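; GA_LeapSlam is a gameplay ability that leaps the character toward the point under the mouse and slams on landing.
; It locks movement, faces the target, then chains jump, fall-loop and land montages through gameplay events, passing the target via SetLeapSlamData.
; On landing, the server multicasts the effect and applies a damage effect to overlapped enemies, while the locally controlled client spawns its own effect.
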(event `self.K2_ActivateAbility`
  (bind _tdwcharacterbase (`self.TDWCharacterBase`))
  (bind (_owneractor _avataractor _playercontroller) (break `GameplayAbilityActorInfo` (`self.GetActorInfo`)))
  (bind (_returnvalue_x _returnvalue_y _returnvalue_z) (`KismetMathLibrary.BreakVector` (`Actor.K2_GetActorLocation` _tdwcharacterbase)))
  (bind (_asynctaskproxy _datahandle) (`TargetDataUnderMouse.CreateTargetDataUnderMouse`)
    (:`ValidData`
      (set `self.TargetLocation` (`.Location` (`GameplayStatics.BreakHitResult` (`AbilitySystemBlueprintLibrary.GetHitResultFromTargetData` _datahandle))))
      (bind _astdwplayer_controller (cast `TDWPlayerController` _playercontroller))
      (bind _output_get (set `self.TDWPlayerController` _astdwplayer_controller))
      (set `TDWPlayerController.bCanMove` false _output_get)
      (bind _astdwcharacter_base (cast `TDWCharacterBase` _avataractor))
      (bind _output_get_2 (set `self.TDWCharacterBase` _astdwcharacter_base))
      (`TDWCharacterBase.SetFacingTarget` _astdwcharacter_base (`self.TargetLocation`))
      (`TDWCharacterBase.SetFacingTarget` _output_get_2 (`self.TargetLocation`))
      (`AbilityTask_PlayMontageAndWait.CreatePlayMontageAndWaitProxy` "None" "/Game/Blueprints/Characters/Mannequins/Animations/Manny/AM_Jump.AM_Jump"
        (:`then`
          (`AbilityTask_WaitGameplayEvent.WaitGameplayEvent` (struct :`TagName` "Event.Montage.JumpStart") null true
            (:`EventReceived`
              (`AbilityTask_PlayMontageAndWait.CreatePlayMontageAndWaitProxy` "None" "/Game/Blueprints/Characters/Mannequins/Animations/Manny/AM_Fall_Loop.AM_Fall_Loop"
                (:`then`
                  (`TDWCharacterBase.SetLeapSlamData` (`self.TDWCharacterBase`) (`self.TargetLocation`))
                  (`AbilityTask_WaitGameplayEvent.WaitGameplayEvent` (struct :`TagName` "Event.Montage.JumpEnd") null true
                    (:`EventReceived`
                      (`AbilityTask_PlayMontageAndWait.CreatePlayMontageAndWaitProxy` "None" "/Game/Blueprints/Characters/Mannequins/Animations/Manny/AM_Land.AM_Land"
                        (:`then`
                          (`AbilityTask_WaitGameplayEvent.WaitGameplayEvent` (struct :`TagName` "Event.Montage.Landing") null true
                            (:`EventReceived`
                              (bind _output_get_3 (set `self.Center` (`KismetMathLibrary.MakeVector` _returnvalue_x _returnvalue_y (- _returnvalue_z (`CapsuleComponent.GetUnscaledCapsuleHalfHeight` (`Character.CapsuleComponent` _tdwcharacterbase))))))
                              (`KismetSystemLibrary.DrawDebugCircle` _output_get_3 200.0 24 (struct :`R` 1.0 :`A` 1.0) 2.0 2.0 (0.0 1.0 0.0) (1.0 0.0 0.0) true)
                              (`self.K2_HasAuthority`
                                (:`True`
                                  (`TDWCharacterBase.Multicast_SpawnSystemAtLocation` (`self.TDWCharacterBase`) (`self.Center`) "/Game/Hack_And_Slash_FX/VFX_Niagara/Slashes/NS_Prestige_Slash.NS_Prestige_Slash")
                                  (bind _outactors (`KismetSystemLibrary.SphereOverlapActors` (`self.Center`) 200.0 (`|MakeArray` "ObjectTypeQuery3" :!type "EObjectTypeQuery Enum") "/Game/Blueprints/Characters/Enemies/BP_TDWEnemyBase.BP_TDWEnemyBase_C"))
                                  (bind _returnvalue (`AbilitySystemBlueprintLibrary.MakeSpecHandleByClass` (`self.DamageClass`)))
                                  (for _array_element _outactors
                                    (`KismetSystemLibrary.PrintString` (`KismetSystemLibrary.GetDisplayName` _array_element))
                                    (`AbilitySystemComponent.BP_ApplyGameplayEffectSpecToSelf` (`AbilitySystemBlueprintLibrary.GetAbilitySystemComponent` _array_element) _returnvalue)))
                                (:`False`
                                  (`self.IsLocallyControlled`
                                    (:`True`
                                      (`NiagaraFunctionLibrary.SpawnSystemAtLocation` "/Game/Hack_And_Slash_FX/VFX_Niagara/Slashes/NS_Prestige_Slash.NS_Prestige_Slash" (`self.Center`)))
                                    (:`False`
                                      _))))
                              (set `TDWPlayerController.bCanMove` true (`self.TDWPlayerController`))
                              (`KismetSystemLibrary.Delay` 0.2)
                              (`self.K2_EndAbility`))))))))))))))))